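; BP_VictoryTimer runs the victory hub screen, counting down before the next level loads.
; On BeginPlay it increments the game instance's score, copies the game mode's general timer, prints lives and score, and plays a victory jingle.
; A looping one-second timer decrements and prints the seconds, then calls LoadLevel on the game instance at zero.
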(event `self.ReceiveBeginPlay`
  (bind _asmain_game_instance (cast `/Game/MainGameInstance` (`GameplayStatics.GetGameInstance`)))
  (bind _result (`/Engine/EditorBlueprintResources/StandardMacros.IncrementInt` (`/Game/MainGameInstance.Score` _asmain_game_instance))
    (:`  `
      (bind _output_get (set `/Game/MainGameInstance.Score` _result _asmain_game_instance))
      (bind _asmain_game_mode (cast `/Game/MainGameMode` (`GameplayStatics.GetGameMode`)))
      (set `self.TimerSeconds` (`/Game/MainGameMode.General_Timer` _asmain_game_mode))
      (`KismetSystemLibrary.PrintString` (`KismetStringLibrary.BuildString_Int` "" "Lives: " (`/Game/MainGameInstance.Lives` _asmain_game_instance)))
      (`KismetSystemLibrary.PrintString` (`KismetStringLibrary.BuildString_Int` "" "Score: " _output_get))
      (`KismetSystemLibrary.K2_SetTimerDelegate` (delegate `ReduceTimer`) 1.0 true)
      (`GameplayStatics.PlaySound2D` "/Game/Sound/WAV_VictoryJingle.WAV_VictoryJingle" 1.0 1.0 0.0 null null))))

(event `ReduceTimer`
  (bind _result (`/Engine/EditorBlueprintResources/StandardMacros.DecrementInt` (`self.TimerSeconds`))
    (:`  `
      (`KismetSystemLibrary.PrintString` (`KismetStringLibrary.BuildString_Int` "" "" _result))
      (if (== (`self.TimerSeconds`) 0)
        (bind _asmain_game_instance (cast `/Game/MainGameInstance` (`GameplayStatics.GetGameInstance`)))
        (`/Game/MainGameInstance.LoadLevel` _asmain_game_instance)))))

(fn `UserConstructionScript`)