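; Game-over screen pawn that plays the game-over sound and lets the player pick between restarting and quitting while a sphere spins.
; Enhanced Input left/right sets Choice and starts a two-second timer for the matching event, with the select sound limited to one play.
; Restart resets score and lives on MainGameInstance and calls its LoadLevel, while the other choice quits the game.
; Only the sound is guarded, so further presses can still set either timer.
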(event `self.ReceiveBeginPlay`
  (bind _asplayer_controller (cast `PlayerController` (`self.GetController`)))
  (`EnhancedInputSubsystemInterface.AddMappingContext` (pcsubsystem `EnhancedInputLocalPlayerSubsystem` _asplayer_controller) "/Game/Input/InputMapping.InputMapping" 0 (struct))
  (`GameplayStatics.PlaySound2D` "/Game/Sound/WAV_GameOver.WAV_GameOver" 1.0 1.0 0.0 null null))

(event `self.ReceiveTick`
  (params (DeltaSeconds :type "Float (single-precision)"))
  (`SceneComponent.K2_AddWorldRotation` (`self.Sphere1`) (`KismetMathLibrary.MakeRotator` 0.0 0.0 (* DeltaSeconds 200.0)) false false))

(event `EnhancedInput|/Game/Input/IA_LeftRight`
  (params (ActionValue :type "Float (double-precision)") (ElapsedSeconds :type "Float (double-precision)") (TriggeredSeconds :type "Float (double-precision)") (InputAction :type "InputAction Object Reference" :default "/Game/Input/IA_LeftRight.IA_LeftRight"))
  (:`Started`
    (if (> ActionValue 0.0)
      (set `self.Choice` 2)
      (`KismetSystemLibrary.K2_SetTimerDelegate` (delegate `ExitGame`) 2.0)
      (if (not (`self.PlayedSound`))
        (`GameplayStatics.PlaySound2D` "/Game/Sound/WAV_Select.WAV_Select" 1.0 0.5 0.0 null null)
        (set `self.PlayedSound` true))
      (else
        (set `self.Choice` 1)
        (`KismetSystemLibrary.K2_SetTimerDelegate` (delegate `ResetGame`) 2.0)
        (if (not (`self.PlayedSound`))
          (`GameplayStatics.PlaySound2D` "/Game/Sound/WAV_Select.WAV_Select" 1.0 2.0 0.0 null null)
          (set `self.PlayedSound` true))))))

(event `ResetGame`
  (bind _asmain_game_instance (cast `/Game/MainGameInstance` (`GameplayStatics.GetGameInstance`)))
  (set `/Game/MainGameInstance.Score` 0 _asmain_game_instance)
  (set `/Game/MainGameInstance.Lives` 4 _asmain_game_instance)
  (`/Game/MainGameInstance.LoadLevel` _asmain_game_instance))

(event `ExitGame`
  (`KismetSystemLibrary.QuitGame` null "Quit"))

(fn `UserConstructionScript`)