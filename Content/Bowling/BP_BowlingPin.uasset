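; BP_BowlingPin is the target pin of a bowling minigame, placed at a random Y position at BeginPlay, when it also resets MainGameMode's WinMinigame flag.
; A capsule overlap with BP_BowlingMC sets that win flag, marks the pin as hit and plays a win sound once.
; Once hit, Tick fakes the knock-away without physics by moving the capsule along X and up while spinning the cylinder.
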(event `self.ReceiveBeginPlay`
  (bind (_returnvalue_x _returnvalue_y _returnvalue_z) (`KismetMathLibrary.BreakVector` (`SceneComponent.K2_GetComponentLocation` (`self.Capsule`))))
  (bind _asmain_game_mode (cast `/Game/MainGameMode` (`GameplayStatics.GetGameMode`)))
  (set `/Game/MainGameMode.WinMinigame` false _asmain_game_mode)
  (`SceneComponent.K2_SetWorldLocation` (`self.Capsule`) (`KismetMathLibrary.MakeVector` _returnvalue_x (`KismetMathLibrary.RandomFloatInRange` -150.0 150.0) _returnvalue_z) false false))

(event `self.ReceiveTick`
  (params (DeltaSeconds :type "Float (single-precision)"))
  (if (`self.Hit`)
    (`SceneComponent.K2_AddWorldOffset` (`self.Capsule`) (`KismetMathLibrary.MakeVector` (* DeltaSeconds 800.0) 0.0 (* DeltaSeconds 1200.0)) false false)
    (`SceneComponent.K2_AddWorldRotation` (`self.Cylinder`) (`KismetMathLibrary.MakeRotator` 0.0 (* DeltaSeconds 2000.0)) false false)))

(event `self.Capsule.OnComponentBeginOverlap`
  (params (OverlappedComponent :type "PrimitiveComponent Object Reference") (OtherActor :type "Actor Object Reference") (OtherComp :type "PrimitiveComponent Object Reference") (OtherBodyIndex :type Integer) (bFromSweep :type Boolean) (SweepResult :type "HitResult Structure (by ref)"))
  (cast `/Game/Bowling/BP_BowlingMC` OtherActor)
  (bind _asmain_game_mode (cast `/Game/MainGameMode` (`GameplayStatics.GetGameMode`)))
  (set `/Game/MainGameMode.WinMinigame` true _asmain_game_mode)
  (`KismetSystemLibrary.PrintString` "Win")
  (set `self.Hit` true)
  (if (not (`self.PlayedSound`))
    (`GameplayStatics.PlaySound2D` "/Game/Sound/WAV_Win.WAV_Win" 1.0 1.0 0.0 null null)
    (set `self.PlayedSound` true)))

(fn `UserConstructionScript`)