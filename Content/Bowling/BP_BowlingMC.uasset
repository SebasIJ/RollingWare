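; BP_BowlingMC is a player-controlled bowling ball that sweeps side to side until the player launches it.
; While aiming, Tick moves the Sphere component along Y, reversing whenever it overlaps a BP_DirectionChanger.
; The Enhanced Input space action sets Roll, switching Tick to constant forward motion along X while Sphere1 spins in pitch to show rolling.
; Movement uses frame-rate-scaled world offsets rather than physics, and Roll is never reset here.
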(event `self.ReceiveBeginPlay`
  (bind _asplayer_controller (cast `PlayerController` (`self.GetController`)))
  (`EnhancedInputSubsystemInterface.AddMappingContext` (pcsubsystem `EnhancedInputLocalPlayerSubsystem` _asplayer_controller) "/Game/Input/InputMapping.InputMapping" 0 (struct)))

(event `self.ReceiveTick`
  (params (DeltaSeconds :type "Float (single-precision)"))
  (if (`self.Roll`)
    (`SceneComponent.K2_AddWorldOffset` (`self.Sphere`) (`KismetMathLibrary.MakeVector` (* DeltaSeconds 700.0)) false false)
    (`SceneComponent.K2_AddWorldRotation` (`self.Sphere1`) (`KismetMathLibrary.MakeRotator` 0.0 (* DeltaSeconds -600.0)) false false)
    (elif (`self.GoRight`)
      (`SceneComponent.K2_AddWorldOffset` (`self.Sphere`) (`KismetMathLibrary.MakeVector` 0.0 (* DeltaSeconds 450.0)) false false)
      (else
        (`SceneComponent.K2_AddWorldOffset` (`self.Sphere`) (`KismetMathLibrary.MakeVector` 0.0 (* DeltaSeconds -450.0)) false false)))))

(event `self.Sphere.OnComponentBeginOverlap`
  (params (OverlappedComponent :type "PrimitiveComponent Object Reference") (OtherActor :type "Actor Object Reference") (OtherComp :type "PrimitiveComponent Object Reference") (OtherBodyIndex :type Integer) (bFromSweep :type Boolean) (SweepResult :type "HitResult Structure (by ref)"))
  (cast `/Game/Bowling/BP_DirectionChanger` OtherActor)
  (set `self.GoRight` (not (`self.GoRight`))))

(event `EnhancedInput|/Game/Input/IA_SpaceAction`
  (params (ActionValue :type Boolean) (ElapsedSeconds :type "Float (double-precision)") (TriggeredSeconds :type "Float (double-precision)") (InputAction :type "InputAction Object Reference" :default "/Game/Input/IA_SpaceAction.IA_SpaceAction"))
  (:`Started`
    (set `self.Roll` true)))

(fn `UserConstructionScript`)