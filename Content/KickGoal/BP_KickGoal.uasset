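; BP_KickGoal is an actor that places its Box component, likely the goal, at a random spot when play begins.
; A random integer selects one of four fixed world positions, equidistant from the world origin along the positive and negative X and Y axes.
; Each case also sets a matching rotation in 90-degree steps.
; Overlap and Tick events are empty, so no scoring or movement logic lives here.
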(event `self.ReceiveBeginPlay`
  (bind _box (`self.Box`))
  (bind _box_2 (`self.Box`))
  (bind _box_3 (`self.Box`))
  (bind _box_4 (`self.Box`))
  (bind _output_get (set `self.Random` (`KismetMathLibrary.RandomIntegerInRange` 0 3)))
  (switch `int` _output_get
    (:`0`
      (`SceneComponent.K2_SetWorldLocation` _box_2 (-900.0 0.0 0.0) false false)
      (`SceneComponent.K2_SetWorldRotation` :`self` _box_2))
    (:`1`
      (`SceneComponent.K2_SetWorldLocation` _box_3 (900.0 0.0 0.0) false false)
      (`SceneComponent.K2_SetWorldRotation` _box_3 (struct :`Yaw` 180.0) false false))
    (:`2`
      (`SceneComponent.K2_SetWorldLocation` _box_4 (0.0 900.0 0.0) false false)
      (`SceneComponent.K2_SetWorldRotation` _box_4 (struct :`Yaw` -90.0) false false))
    (:`3`
      (`SceneComponent.K2_SetWorldLocation` _box (0.0 -900.0 0.0) false false)
      (`SceneComponent.K2_SetWorldRotation` _box (struct :`Yaw` 90.0) false false))))

(fn `UserConstructionScript`)