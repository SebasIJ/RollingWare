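; Player-controlled ball for the KickGoal minigame, which the player must launch toward the goal.
; A looping timer turns the ball's aim in short stepped bursts on Tick until the Space input action sets it rolling.
; While rolling, Tick moves it forward without sweep and spins the inner sphere.
; Any overlap stops it, but only hitting BP_KickGoal flags the win on MainGameMode and plays the win sound once.
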(event `self.ReceiveBeginPlay`
  (bind _asplayer_controller (cast `PlayerController` (`self.GetController`)))
  (`EnhancedInputSubsystemInterface.AddMappingContext` (pcsubsystem `EnhancedInputLocalPlayerSubsystem` _asplayer_controller) "/Game/Input/InputMapping.InputMapping" 0 (struct))
  (`KismetSystemLibrary.K2_SetTimerDelegate` (delegate `Spin`) 1.0 true))

(event `Spin`
  (if (not (`self.Roll`))
    (set `self.Spinning` true)))

(event `self.ReceiveTick`
  (params (DeltaSeconds :type "Float (single-precision)"))
  (if (`self.Goal`)
    _
    (elif (`self.Roll`)
      (`SceneComponent.K2_AddWorldOffset` (`self.Sphere`) (* (`SceneComponent.GetForwardVector` (`self.Sphere`)) (* DeltaSeconds 800)) false false)
      (`SceneComponent.K2_AddLocalRotation` (`self.Sphere1`) (`KismetMathLibrary.MakeRotator` 0.0 (* DeltaSeconds -800.0)) false false)
      (elif (`self.Spinning`)
        (`SceneComponent.K2_AddWorldRotation` (`self.Sphere`) (`KismetMathLibrary.MakeRotator` 0.0 0.0 10.0) false false)
        (bind _result (`/Engine/EditorBlueprintResources/StandardMacros.IncrementInt` (`self.Counter`))
          (:`  `
            (if (== _result 9)
              (set `self.Spinning` false)
              (set `self.Counter` 0))))))))

(event `EnhancedInput|/Game/Input/IA_SpaceAction`
  (params (ActionValue :type Boolean) (ElapsedSeconds :type "Float (double-precision)") (TriggeredSeconds :type "Float (double-precision)") (InputAction :type "InputAction Object Reference" :default "/Game/Input/IA_SpaceAction.IA_SpaceAction"))
  (:`Started`
    (set `self.Roll` true)))

(event `self.Sphere.OnComponentBeginOverlap`
  (params (OverlappedComponent :type "PrimitiveComponent Object Reference") (OtherActor :type "Actor Object Reference") (OtherComp :type "PrimitiveComponent Object Reference") (OtherBodyIndex :type Integer) (bFromSweep :type Boolean) (SweepResult :type "HitResult Structure (by ref)"))
  (cast `/Game/KickGoal/BP_KickGoal` OtherActor
    (:`then`
      (set `self.Goal` true)
      (bind _asmain_game_mode (cast `/Game/MainGameMode` (`GameplayStatics.GetGameMode`)))
      (set `/Game/MainGameMode.WinMinigame` true _asmain_game_mode)
      (if (not (`self.PlayedSound`))
        (`GameplayStatics.PlaySound2D` "/Game/Sound/WAV_Win.WAV_Win" 1.0 1.0 0.0 null null)
        (set `self.PlayedSound` true)))
    (:`CastFailed`
      (set `self.Goal` true))))

(fn `UserConstructionScript`)