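; BP_CleanTimer is the countdown actor for the CleanBall minigame that decides its win or lose outcome.
; On BeginPlay it clears WinMinigame on MainGameMode, copies GeneralTimer as the starting seconds, and starts a one-second looping timer.
; Each tick decrements and prints the count; at zero it reads WinMinigame and opens either the victory or failure hub level.
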(event `self.ReceiveBeginPlay`
  (bind _asmain_game_mode (cast `/Game/MainGameMode` (`GameplayStatics.GetGameMode`)))
  (set `/Game/MainGameMode.WinMinigame` false _asmain_game_mode)
  (set `self.TimerSeconds` (`/Game/MainGameMode.General_Timer` _asmain_game_mode))
  (`KismetSystemLibrary.K2_SetTimerDelegate` (delegate `ReduceTimer`) 1.0 true))

(event `ReduceTimer`
  (bind _result (`/Engine/EditorBlueprintResources/StandardMacros.DecrementInt` (`self.TimerSeconds`))
    (:`  `
      (`KismetSystemLibrary.PrintString` (`KismetStringLibrary.BuildString_Int` "" "" _result))
      (if (== (`self.TimerSeconds`) 0)
        (bind _asmain_game_mode (cast `/Game/MainGameMode` (`GameplayStatics.GetGameMode`)))
        (if (`/Game/MainGameMode.WinMinigame` _asmain_game_mode)
          (`KismetSystemLibrary.PrintString` "Win")
          (`GameplayStatics.OpenLevelBySoftObjectPtr` "/Game/VictoryHub/LV_VictoryHub.LV_VictoryHub")
          (else
            (`KismetSystemLibrary.PrintString` "Lose")
            (`GameplayStatics.OpenLevelBySoftObjectPtr` "/Game/FailureHub/LV_FailureHub.LV_FailureHub")))))))

(fn `UserConstructionScript`)