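; BP_Sponge is a player-controlled sponge in CleanBall that shifts sideways between a left and a right position.
; BeginPlay adds the input mapping context, and IA_LeftRight starts a move only toward the opposite side when none is in progress.
; Tick slides the Box in fixed, unswept steps over a few frames, then records the side reached, so movement speed depends on frame rate.
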(event `self.ReceiveBeginPlay`
  (bind _asplayer_controller (cast `PlayerController` (`self.GetController`)))
  (`EnhancedInputSubsystemInterface.AddMappingContext` (pcsubsystem `EnhancedInputLocalPlayerSubsystem` _asplayer_controller) "/Game/Input/InputMapping.InputMapping" 0 (struct)))

(event `self.ReceiveTick`
  (params (DeltaSeconds :type "Float (single-precision)"))
  (if (`self.Move`)
    (if (`self.Right`)
      (`SceneComponent.K2_AddLocalOffset` (`self.Box`) (0.0 30.0 0.0) false false)
      (bind _result (`/Engine/EditorBlueprintResources/StandardMacros.IncrementInt` (`self.Counter`))
        (:`  `
          (if (== _result 3)
            (set `self.Move` false)
            (set `self.Counter` 0)
            (set `self.LastRight` true))))
      (else
        (`SceneComponent.K2_AddLocalOffset` (`self.Box`) (0.0 -30.0 0.0) false false)
        (bind _result_2 (`/Engine/EditorBlueprintResources/StandardMacros.IncrementInt` (`self.Counter`))
          (:`  `
            (if (== _result_2 3)
              (set `self.Move` false)
              (set `self.Counter` 0)
              (set `self.LastRight` false))))))))

(event `EnhancedInput|/Game/Input/IA_LeftRight`
  (params (ActionValue :type "Float (double-precision)") (ElapsedSeconds :type "Float (double-precision)") (TriggeredSeconds :type "Float (double-precision)") (InputAction :type "InputAction Object Reference" :default "/Game/Input/IA_LeftRight.IA_LeftRight"))
  (bind _lastright (`self.LastRight`))
  (:`Started`
    (if (== (`self.Counter`) 0)
      (if (> ActionValue 0.0)
        (if (not _lastright)
          (set `self.Right` true)
          (set `self.Move` true))
        (elif _lastright
          (set `self.Right` false)
          (set `self.Move` true))))))

(fn `UserConstructionScript`)