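; BP_CleanBallMC is a ball-cleaning minigame actor with a spot sprite that a sponge wipes away.
; On BeginPlay it randomizes the sphere's yaw and the cleaning strength of each pass.
; Each sponge overlap with the Box lowers the spot's alpha by that strength.
; When the spot becomes fully transparent, it flags the minigame as won on MainGameMode and plays a win sound once.
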(event `self.ReceiveBeginPlay`
  (`SceneComponent.K2_SetRelativeRotation` (`self.Sphere1`) (`KismetMathLibrary.MakeRotator` 0.0 0.0 (`KismetMathLibrary.RandomFloatInRange` -180.0 180.0)) false false)
  (set `self.CleanPower` (`KismetMathLibrary.RandomFloatInRange` 0.06 0.08)))

(event `self.Box.OnComponentBeginOverlap`
  (params (OverlappedComponent :type "PrimitiveComponent Object Reference") (OtherActor :type "Actor Object Reference") (OtherComp :type "PrimitiveComponent Object Reference") (OtherBodyIndex :type Integer) (bFromSweep :type Boolean) (SweepResult :type "HitResult Structure (by ref)"))
  (bind _spot (`self.Spot`))
  (bind (_spritecolor_r _spritecolor_g _spritecolor_b _spritecolor_a) (break `LinearColor` (`PaperSpriteComponent.SpriteColor` _spot)))
  (bind (_spritecolor_r_2 _spritecolor_g_2 _spritecolor_b_2 _spritecolor_a_2) (break `LinearColor` (`PaperSpriteComponent.SpriteColor` _spot)))
  (cast `/Game/CleanBall/BP_Sponge` OtherActor)
  (`PaperSpriteComponent.SetSpriteColor` _spot (make `LinearColor` _spritecolor_r _spritecolor_g _spritecolor_b (- _spritecolor_a (`self.CleanPower`))))
  (if (<= _spritecolor_a_2 0.0)
    (bind _asmain_game_mode (cast `/Game/MainGameMode` (`GameplayStatics.GetGameMode`)))
    (set `/Game/MainGameMode.WinMinigame` true _asmain_game_mode)
    (if (not (`self.PlayedSound`))
      (`GameplayStatics.PlaySound2D` "/Game/Sound/WAV_Win.WAV_Win" 1.0 1.0 0.0 null null)
      (set `self.PlayedSound` true))))

(fn `UserConstructionScript`)