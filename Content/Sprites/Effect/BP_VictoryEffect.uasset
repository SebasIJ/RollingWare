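; BP_VictoryEffect is a flipbook effect actor that plays a victory animation when the minigame is won.
; BeginPlay freezes the flipbook at zero play rate and turns off looping.
; Tick polls MainGameMode's WinMinigame flag and restores normal play rate once it is true.
; The poll is gated by a Played flag, which this Blueprint reads but never sets.
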(event `self.ReceiveBeginPlay`
  (bind _paperflipbook (`self.PaperFlipbook`))
  (`PaperFlipbookComponent.SetPlayRate` _paperflipbook 0.0)
  (`PaperFlipbookComponent.SetLooping` _paperflipbook false))

(event `self.ReceiveTick`
  (params (DeltaSeconds :type "Float (single-precision)"))
  (if (not (`self.Played`))
    (bind _asmain_game_mode (cast `/Game/MainGameMode` (`GameplayStatics.GetGameMode`)))
    (if (`/Game/MainGameMode.WinMinigame` _asmain_game_mode)
      (`PaperFlipbookComponent.SetPlayRate` (`self.PaperFlipbook`) 1.0))))

(fn `UserConstructionScript`)