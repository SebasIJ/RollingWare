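; Title screen pawn that shows a constantly spinning sphere and starts the game on the Space input action.
; BeginPlay adds its Enhanced Input mapping context, and Tick spins Sphere1 and, once started, moves Sphere along its local X axis.
; The input plays a select sound once and sets a timer that calls LoadLevel on MainGameInstance.
; A separate event toggles visibility of the Arrow and Sphere components for debugging.
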(event `self.ReceiveBeginPlay`
  (bind _asplayer_controller (cast `PlayerController` (`self.GetController`)))
  (`EnhancedInputSubsystemInterface.AddMappingContext` (pcsubsystem `EnhancedInputLocalPlayerSubsystem` _asplayer_controller) "/Game/Input/InputMapping.InputMapping" 0 (struct)))

(event `self.ReceiveTick`
  (params (DeltaSeconds :type "Float (single-precision)"))
  (`SceneComponent.K2_AddLocalRotation` (`self.Sphere1`) (`KismetMathLibrary.MakeRotator` 0.0 (* DeltaSeconds -300.0)) false false)
  (if (`self.Started`)
    (`SceneComponent.K2_AddLocalOffset` (`self.Sphere`) (`KismetMathLibrary.MakeVector` (* DeltaSeconds 300.0)) false false)))

(event `EnhancedInput|/Game/Input/IA_SpaceAction`
  (params (ActionValue :type Boolean) (ElapsedSeconds :type "Float (double-precision)") (TriggeredSeconds :type "Float (double-precision)") (InputAction :type "InputAction Object Reference" :default "/Game/Input/IA_SpaceAction.IA_SpaceAction"))
  (:`Started`
    (set `self.Started` true)
    (`KismetSystemLibrary.K2_SetTimerDelegate` (delegate `LoadLevel`) 3.0)
    (if (not (`self.SoundPlayed`))
      (`GameplayStatics.PlaySound2D` "/Game/Sound/WAV_Select.WAV_Select" 1.0 2.0 0.0 null null)
      (set `self.SoundPlayed` true))))

(event `LoadLevel`
  (bind _asmain_game_instance (cast `/Game/MainGameInstance` (`GameplayStatics.GetGameInstance`)))
  (`/Game/MainGameInstance.LoadLevel` _asmain_game_instance))

(event `/Game/I_ToggeableDebugVisualization.ToggleDebugVisualization`
  (if (`self.ToggleOn`)
    (`SceneComponent.SetHiddenInGame` (`self.Arrow`) true false)
    (`SceneComponent.SetHiddenInGame` (`self.Sphere`) true false)
    (set `self.ToggleOn` false)
    (else
      (`SceneComponent.SetHiddenInGame` (`self.Arrow`) false false)
      (`SceneComponent.SetHiddenInGame` (`self.Sphere`) false false)
      (set `self.ToggleOn` true))))

(fn `UserConstructionScript`)