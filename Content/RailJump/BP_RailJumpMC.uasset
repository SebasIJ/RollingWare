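; BP_RailJumpMC is the player character of the RailJump minigame, jumping on a key press and losing if it falls.
; BeginPlay adds the input mapping and presets MainGameMode's WinMinigame to true; Tick spins Sphere1 and clears that flag below a height threshold.
; Jumps use LaunchCharacter with a sound, gated by a Landed flag that capsule hits set and jumping or leaving a BP_RailConfig1 overlap clears.
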(event `self.ReceiveBeginPlay`
  (bind _asplayer_controller (cast `PlayerController` (`self.GetController`)))
  (`EnhancedInputSubsystemInterface.AddMappingContext` (pcsubsystem `EnhancedInputLocalPlayerSubsystem` _asplayer_controller) "/Game/Input/InputMapping.InputMapping" 0 (struct))
  (bind _asmain_game_mode (cast `/Game/MainGameMode` (`GameplayStatics.GetGameMode`)))
  (set `/Game/MainGameMode.WinMinigame` true _asmain_game_mode))

(event `self.ReceiveTick`
  (params (DeltaSeconds :type "Float (single-precision)"))
  (bind (_returnvalue_x _returnvalue_y _returnvalue_z) (`KismetMathLibrary.BreakVector` (`self.K2_GetActorLocation`)))
  (`SceneComponent.K2_AddLocalRotation` (`self.Sphere1`) (struct :`Pitch` -5.0) false false)
  (if (< _returnvalue_z -100.0)
    (bind _asmain_game_mode (cast `/Game/MainGameMode` (`GameplayStatics.GetGameMode`)))
    (set `/Game/MainGameMode.WinMinigame` false _asmain_game_mode)))

(event `EnhancedInput|/Game/Input/IA_SpaceAction`
  (params (ActionValue :type Boolean) (ElapsedSeconds :type "Float (double-precision)") (TriggeredSeconds :type "Float (double-precision)") (InputAction :type "InputAction Object Reference" :default "/Game/Input/IA_SpaceAction.IA_SpaceAction"))
  (:`Started`
    (if (`self.Landed`)
      (`self.LaunchCharacter` (* (`self.GetActorUpVector`) 600.0) false true)
      (set `self.Landed` false)
      (`GameplayStatics.PlaySound2D` "/Game/Sound/WAV_Jump.WAV_Jump" 1.0 1.0 0.0 null null))))

(event `self.CapsuleComponent.OnComponentHit`
  (params (HitComponent :type "PrimitiveComponent Object Reference") (OtherActor :type "Actor Object Reference") (OtherComp :type "PrimitiveComponent Object Reference") (NormalImpulse :type "Vector Structure") (Hit :type "HitResult Structure (by ref)"))
  (set `self.Landed` true))

(event `self.CapsuleComponent.OnComponentEndOverlap`
  (params (OverlappedComponent :type "PrimitiveComponent Object Reference") (OtherActor :type "Actor Object Reference") (OtherComp :type "PrimitiveComponent Object Reference") (OtherBodyIndex :type Integer))
  (cast `/Game/RailJump/BP_RailConfig1` OtherActor)
  (set `self.Landed` false))

(fn `UserConstructionScript`)