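; BP_RailConfig1 is a moving rail segment for RailJump that chains an endless track by spawning copies of itself.
; Every tick it offsets its root along local X at Speed.
; When BP_RailJumpMC overlaps RailBeginning, it spawns the next segment beyond RailEnd on world X, keeping Y and Z.
; The new segment gets a random X scale, and its spawn distance adds a randomized offset to a fixed gap.
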(event `self.ReceiveBeginPlay`)

(event `self.ReceiveTick`
  (params (DeltaSeconds :type "Float (single-precision)"))
  (`SceneComponent.K2_AddLocalOffset` (`self.DefaultSceneRoot`) (`KismetMathLibrary.MakeVector` (* (`self.Speed`) DeltaSeconds)) false false))

(event `self.RailBeginning.OnComponentBeginOverlap`
  (params (OverlappedComponent :type "PrimitiveComponent Object Reference") (OtherActor :type "Actor Object Reference") (OtherComp :type "PrimitiveComponent Object Reference") (OtherBodyIndex :type Integer) (bFromSweep :type Boolean) (SweepResult :type "HitResult Structure (by ref)"))
  (bind _returnvalue (`KismetMathLibrary.RandomFloatInRange` 0.15 0.5))
  (bind (_returnvalue_x _returnvalue_y _returnvalue_z) (`KismetMathLibrary.BreakVector` (`SceneComponent.K2_GetComponentLocation` (`self.DefaultSceneRoot`))))
  (bind _returnvalue_x_2 (`KismetMathLibrary.BreakVector` (`SceneComponent.K2_GetComponentLocation` (`self.RailEnd`))))
  (cast `/Game/RailJump/BP_RailJumpMC` OtherActor)
  (`|SpawnActorFromClass` "BP_RailConfig1_C" (`KismetMathLibrary.MakeTransform` (`KismetMathLibrary.MakeVector` (+ (+ _returnvalue_x_2 (* 600.0 _returnvalue)) 250.0) _returnvalue_y _returnvalue_z) (struct) (`KismetMathLibrary.MakeVector` _returnvalue 1.0 1.0)) "Undefined" "MultiplyWithRoot" null null))

(fn `UserConstructionScript`)