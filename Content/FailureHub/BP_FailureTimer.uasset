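; BP_FailureTimer runs the failure interlude between levels, charging a life and counting down to the next load.
; On BeginPlay it decrements Lives on MainGameInstance, prints lives and score, plays a lose jingle and takes the countdown length from MainGameMode's GeneralTimer.
; A looping one-second timer prints the countdown, then at zero calls LoadLevel on the game instance, or opens LV_GameOver when no lives remain.
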(event `self.ReceiveBeginPlay`
  (bind _asmain_game_instance (cast `/Game/MainGameInstance` (`GameplayStatics.GetGameInstance`)))
  (bind _result (`/Engine/EditorBlueprintResources/StandardMacros.DecrementInt` (`/Game/MainGameInstance.Lives` _asmain_game_instance))
    (:`  `
      (bind _output_get (set `/Game/MainGameInstance.Lives` _result _asmain_game_instance))
      (bind _asmain_game_mode (cast `/Game/MainGameMode` (`GameplayStatics.GetGameMode`)))
      (set `self.TimerSeconds` (`/Game/MainGameMode.General_Timer` _asmain_game_mode))
      (`KismetSystemLibrary.PrintString` (`KismetStringLibrary.BuildString_Int` "" "Lives: " _output_get))
      (`KismetSystemLibrary.PrintString` (`KismetStringLibrary.BuildString_Int` "" "Score: " (`/Game/MainGameInstance.Score` _asmain_game_instance)))
      (`KismetSystemLibrary.K2_SetTimerDelegate` (delegate `ReduceTimer`) 1.0 true)
      (`GameplayStatics.PlaySound2D` "/Game/Sound/WAV_LoseJingle.WAV_LoseJingle" 1.0 1.0 0.0 null null))))

(event `ReduceTimer`
  (bind _result (`/Engine/EditorBlueprintResources/StandardMacros.DecrementInt` (`self.TimerSeconds`))
    (:`  `
      (`KismetSystemLibrary.PrintString` (`KismetStringLibrary.BuildString_Int` "" "" _result))
      (if (== (`self.TimerSeconds`) 0)
        (bind _asmain_game_instance (cast `/Game/MainGameInstance` (`GameplayStatics.GetGameInstance`)))
        (if (> (`/Game/MainGameInstance.Lives` _asmain_game_instance) 0)
          (`/Game/MainGameInstance.LoadLevel` _asmain_game_instance)
          (else
            (`GameplayStatics.OpenLevelBySoftObjectPtr` "/Game/GameOver/LV_GameOver.LV_GameOver")))))))

(fn `UserConstructionScript`)