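; Player character for the target landing minigame, steered as it descends toward a landing platform.
; Enhanced Input axes add movement along the actor's right and forward vectors and tilt Sphere1, which resets upright when input ends.
; A capsule hit sets Landed, which stops steering, and flags the landing in MainGameMode, also marking a win if the hit actor is a BP_LandingPlatform.
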(event `self.ReceiveBeginPlay`
  (bind _asplayer_controller (cast `PlayerController` (`self.GetController`)))
  (`EnhancedInputSubsystemInterface.AddMappingContext` (pcsubsystem `EnhancedInputLocalPlayerSubsystem` _asplayer_controller) "/Game/Input/InputMapping.InputMapping" 0 (struct)))

(event `EnhancedInput|/Game/Input/IA_LeftRight`
  (params (ActionValue :type "Float (double-precision)") (ElapsedSeconds :type "Float (double-precision)") (TriggeredSeconds :type "Float (double-precision)") (InputAction :type "InputAction Object Reference" :default "/Game/Input/IA_LeftRight.IA_LeftRight"))
  (bind _returnvalue (* ActionValue 90.0))
  (:`Triggered`
    (if (not (`self.Landed`))
      (`self.AddMovementInput` (`self.GetActorRightVector`) ActionValue)
      (`SceneComponent.K2_SetWorldRotation` (`self.Sphere1`) (`KismetMathLibrary.MakeRotator` _returnvalue (+ 30.0 -90.0) (* _returnvalue -1.0)) false false)))
  (:`Canceled`
    (`SceneComponent.K2_SetWorldRotation` (`self.Sphere1`) (`KismetMathLibrary.MakeRotator` 0.0 -90.0) false false :!label _label))
  (:`Completed`
    (goto _label)))

(event `EnhancedInput|/Game/Input/IA_UpDown`
  (params (ActionValue :type "Float (double-precision)") (ElapsedSeconds :type "Float (double-precision)") (TriggeredSeconds :type "Float (double-precision)") (InputAction :type "InputAction Object Reference" :default "/Game/Input/IA_UpDown.IA_UpDown"))
  (:`Triggered`
    (if (not (`self.Landed`))
      (`self.AddMovementInput` (`self.GetActorForwardVector`) ActionValue)
      (`SceneComponent.K2_SetWorldRotation` (`self.Sphere1`) (`KismetMathLibrary.MakeRotator` 0.0 (+ (* ActionValue -30.0) -90.0)) false false)))
  (:`Canceled`
    (`SceneComponent.K2_SetWorldRotation` (`self.Sphere1`) (`KismetMathLibrary.MakeRotator` 0.0 -90.0) false false :!label _label_2))
  (:`Completed`
    (goto _label_2)))

(event `self.CapsuleComponent.OnComponentHit`
  (params (HitComponent :type "PrimitiveComponent Object Reference") (OtherActor :type "Actor Object Reference") (OtherComp :type "PrimitiveComponent Object Reference") (NormalImpulse :type "Vector Structure") (Hit :type "HitResult Structure (by ref)"))
  (set `self.Landed` true)
  (bind _asmain_game_mode (cast `/Game/MainGameMode` (`GameplayStatics.GetGameMode`)))
  (set `/Game/MainGameMode.LandingMin_PlayerLand` true _asmain_game_mode)
  (cast `/Game/TargetLanding/BP_LandingPlatform` OtherActor)
  (set `/Game/MainGameMode.WinMinigame` true _asmain_game_mode))

(fn `UserConstructionScript`)