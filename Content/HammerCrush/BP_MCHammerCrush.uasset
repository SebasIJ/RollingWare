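; Player pawn for the Hammer Crush minigame, where the player moves sideways to avoid being crushed by hammers.
; Enhanced Input drives left/right movement and rolls a sphere component to match, as long as the pawn is not crushed.
; The minigame counts as won from BeginPlay; overlapping a BP_Hammers flattens the sphere, locks movement and flags MainGameMode's WinMinigame as lost.
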(event `self.ReceiveBeginPlay`
  (bind _asplayer_controller (cast `PlayerController` (`self.GetController`)))
  (`EnhancedInputSubsystemInterface.AddMappingContext` (pcsubsystem `EnhancedInputLocalPlayerSubsystem` _asplayer_controller) "/Game/Input/InputMapping.InputMapping" 0 (struct))
  (set `self.NotCrushed` true)
  (bind _asmain_game_mode (cast `/Game/MainGameMode` (`GameplayStatics.GetGameMode`)))
  (set `/Game/MainGameMode.WinMinigame` true _asmain_game_mode))

(event `EnhancedInput|/Game/Input/IA_LeftRight`
  (params (ActionValue :type "Float (double-precision)") (ElapsedSeconds :type "Float (double-precision)") (TriggeredSeconds :type "Float (double-precision)") (InputAction :type "InputAction Object Reference" :default "/Game/Input/IA_LeftRight.IA_LeftRight"))
  (bind _returnvalue (* ActionValue -1.0))
  (:`Triggered`
    (if (`self.NotCrushed`)
      (`self.AddMovementInput` (`self.GetActorRightVector`) _returnvalue)
      (`SceneComponent.K2_AddWorldRotation` (`self.Sphere1`) (`KismetMathLibrary.MakeRotator` (* _returnvalue 10.0)) false false))))

(event `self.Sphere.OnComponentBeginOverlap`
  (params (OverlappedComponent :type "PrimitiveComponent Object Reference") (OtherActor :type "Actor Object Reference") (OtherComp :type "PrimitiveComponent Object Reference") (OtherBodyIndex :type Integer) (bFromSweep :type Boolean) (SweepResult :type "HitResult Structure (by ref)"))
  (if (`self.NotCrushed`)
    (cast `/Game/HammerCrush/BP_Hammers` OtherActor)
    (set `self.NotCrushed` false)
    (`SceneComponent.SetWorldScale3D` (`self.Sphere`) (2.0 2.0 0.01))
    (`SceneComponent.K2_SetWorldRotation` :`self` (`self.Sphere1`))
    (`SceneComponent.K2_AddWorldOffset` (`self.Sphere`) (0.0 0.0 -25.0) false false)
    (bind _asmain_game_mode (cast `/Game/MainGameMode` (`GameplayStatics.GetGameMode`)))
    (set `/Game/MainGameMode.WinMinigame` false _asmain_game_mode)))

(fn `UserConstructionScript`)