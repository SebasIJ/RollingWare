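; BP_Hammers drives a crushing hammer, Hammer1, that shakes as a wind-up, then slams down.
; A looping fast timer runs WorkHammer while Ready is false, and ShakeHammer counts ticks while Charging, jolting the hammer vertically every third count.
; At the count limit it drops instantly with a 2D sound.
; A delayed RaiseHammer restores its height and sets Ready, which halts the cycle; nothing here clears that flag.
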(event `self.ReceiveBeginPlay`
  (bind _hammer1 (`self.Hammer1`))
  (bind (_returnvalue_x _returnvalue_y) (`KismetMathLibrary.BreakVector` (`SceneComponent.K2_GetComponentLocation` _hammer1)))
  (`SceneComponent.K2_SetWorldLocation` _hammer1 (`KismetMathLibrary.MakeVector` _returnvalue_x _returnvalue_y 380.0) false false)
  (`KismetSystemLibrary.K2_SetTimerDelegate` (delegate `WorkHammer`) 0.015 true))

(event `WorkHammer`
  (if (`self.Ready`)
    _
    (elif (== (`self.ShakeCount`) 50)
      (`SceneComponent.K2_AddWorldOffset` (`self.Hammer1`) (0.0 0.0 -200.0) false false)
      (set `self.Charging` false)
      (set `self.ShakeCount` 0)
      (`KismetSystemLibrary.K2_SetTimerDelegate` (delegate `Raise Hammer`) 1.0)
      (`GameplayStatics.PlaySound2D` "/Game/Sound/WAV_Hammer.WAV_Hammer" 1.0 1.0 0.0 null null)
      (else
        (`self.ShakeHammer`)))))

(event `self.ReceiveTick`
  (params (DeltaSeconds :type "Float (single-precision)")))

(event `Raise Hammer`
  (bind _hammer1 (`self.Hammer1`))
  (bind (_returnvalue_x _returnvalue_y) (`KismetMathLibrary.BreakVector` (`SceneComponent.K2_GetComponentLocation` _hammer1)))
  (`SceneComponent.K2_SetWorldLocation` _hammer1 (`KismetMathLibrary.MakeVector` _returnvalue_x _returnvalue_y 380.0) false false)
  (set `self.Ready` true)
  (set `self.Charging` true)
  (set `self.Up` false))

(fn `ShakeHammer`
  (if (`self.Charging`)
    (bind _result (`/Engine/EditorBlueprintResources/StandardMacros.IncrementInt` (`self.ShakeCount`))
      (:`  `
        (if (== (mod _result 3) 0)
          (if (`self.Up`)
            (`SceneComponent.K2_AddWorldOffset` (`self.Hammer1`) (0.0 0.0 10.0) false false)
            (set `self.Up` false)
            (else
              (`SceneComponent.K2_AddWorldOffset` (`self.Hammer1`) (0.0 0.0 -10.0) false false)
              (set `self.Up` true))))))))

(fn `UserConstructionScript`)