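; Player pawn for a coin-collecting minigame, moved with Enhanced Input while its Sphere1 component rotates to mimic rolling.
; Sphere overlaps destroy BP_Coin actors, count them and play a coin sound.
; When the count matches the total read from MainGameMode at BeginPlay, it sets WinMinigame on that game mode and plays a win sound once.
; A helper function toggles visibility of the Arrow and Sphere for debugging.
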(event `self.ReceiveBeginPlay`
  (bind _asplayer_controller (cast `PlayerController` (`self.GetController`)))
  (`EnhancedInputSubsystemInterface.AddMappingContext` (pcsubsystem `EnhancedInputLocalPlayerSubsystem` _asplayer_controller) "/Game/Input/InputMapping.InputMapping" 0 (struct))
  (bind _asmain_game_mode (cast `/Game/MainGameMode` (`GameplayStatics.GetGameMode`)))
  (set `self.TotalCoins` (`/Game/MainGameMode.CoinMin_TotalCoins` _asmain_game_mode))
  (set `self.CoinCount` 0))

(event `EnhancedInput|/Game/Input/IA_LeftRight`
  (params (ActionValue :type "Float (double-precision)") (ElapsedSeconds :type "Float (double-precision)") (TriggeredSeconds :type "Float (double-precision)") (InputAction :type "InputAction Object Reference" :default "/Game/Input/IA_LeftRight.IA_LeftRight"))
  (:`Triggered`
    (`self.AddMovementInput` (`self.GetActorRightVector`) ActionValue)
    (`SceneComponent.K2_AddWorldRotation` (`self.Sphere1`) (`KismetMathLibrary.MakeRotator` (* ActionValue 10.0)) false false)))

(event `EnhancedInput|/Game/Input/IA_UpDown`
  (params (ActionValue :type "Float (double-precision)") (ElapsedSeconds :type "Float (double-precision)") (TriggeredSeconds :type "Float (double-precision)") (InputAction :type "InputAction Object Reference" :default "/Game/Input/IA_UpDown.IA_UpDown"))
  (:`Triggered`
    (`self.AddMovementInput` (`self.GetActorForwardVector`) ActionValue)
    (`SceneComponent.K2_AddWorldRotation` (`self.Sphere1`) (`KismetMathLibrary.MakeRotator` 0.0 (* ActionValue -10.0)) false false)))

(event `self.Sphere.OnComponentBeginOverlap`
  (params (OverlappedComponent :type "PrimitiveComponent Object Reference") (OtherActor :type "Actor Object Reference") (OtherComp :type "PrimitiveComponent Object Reference") (OtherBodyIndex :type Integer) (bFromSweep :type Boolean) (SweepResult :type "HitResult Structure (by ref)"))
  (bind _asbp_coin (cast `/Game/CoinGet/BP_Coin` OtherActor))
  (bind _result (`/Engine/EditorBlueprintResources/StandardMacros.IncrementInt` (`self.CoinCount`))
    (:`  `
      (set `self.CoinCount` _result)
      (`self.K2_DestroyActor` _asbp_coin)
      (`KismetSystemLibrary.PrintString` (`KismetStringLibrary.BuildString_Int` "" "" (`self.CoinCount`)))
      (if (== (`self.CoinCount`) (`self.TotalCoins`))
        (`KismetSystemLibrary.PrintString` "GameWon")
        (bind _asmain_game_mode (cast `/Game/MainGameMode` (`GameplayStatics.GetGameMode`)))
        (set `/Game/MainGameMode.WinMinigame` true _asmain_game_mode)
        (if (not (`self.PlayedSound`))
          (`GameplayStatics.PlaySound2D` "/Game/Sound/WAV_Win.WAV_Win" 1.0 1.0 0.0 null null)
          (set `self.PlayedSound` true))
        (else
          (`GameplayStatics.PlaySound2D` "/Game/Sound/WAV_Coin.WAV_Coin" 1.0 1.0 0.0 null null))))))

(fn `ToggleDebugVisualization`
  (if (`self.ToggleOn`)
    (`SceneComponent.SetHiddenInGame` (`self.Arrow`) true false)
    (`SceneComponent.SetHiddenInGame` (`self.Sphere`) true false)
    (set `self.ToggleOn` false)
    (else
      (`SceneComponent.SetHiddenInGame` (`self.Arrow`) false false)
      (`SceneComponent.SetHiddenInGame` (`self.Sphere`) false false)
      (set `self.ToggleOn` true)))
  (return))

(fn `UserConstructionScript`)