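; Player character for the car dodge minigame, a ball that rolls around and gets squashed by cars.
; Enhanced Input axes drive movement input and spin the Sphere1 component to fake rolling while NotCrushed is true.
; Overlapping a BP_Car clears that flag, stopping control, and flattens the collision Sphere while resetting Sphere1's rotation.
; A ToggleDebugVisualization event shows or hides the Arrow and Sphere.
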(event `self.ReceiveBeginPlay`
  (bind _asplayer_controller (cast `PlayerController` (`self.GetController`)))
  (`EnhancedInputSubsystemInterface.AddMappingContext` (pcsubsystem `EnhancedInputLocalPlayerSubsystem` _asplayer_controller) "/Game/Input/InputMapping.InputMapping" 0 (struct))
  (set `self.NotCrushed` true))

(event `EnhancedInput|/Game/Input/IA_LeftRight`
  (params (ActionValue :type "Float (double-precision)") (ElapsedSeconds :type "Float (double-precision)") (TriggeredSeconds :type "Float (double-precision)") (InputAction :type "InputAction Object Reference" :default "/Game/Input/IA_LeftRight.IA_LeftRight"))
  (:`Triggered`
    (if (`self.NotCrushed`)
      (`self.AddMovementInput` (`self.GetActorRightVector`) ActionValue)
      (`SceneComponent.K2_AddWorldRotation` (`self.Sphere1`) (`KismetMathLibrary.MakeRotator` (* ActionValue 10.0)) false false))))

(event `EnhancedInput|/Game/Input/IA_UpDown`
  (params (ActionValue :type "Float (double-precision)") (ElapsedSeconds :type "Float (double-precision)") (TriggeredSeconds :type "Float (double-precision)") (InputAction :type "InputAction Object Reference" :default "/Game/Input/IA_UpDown.IA_UpDown"))
  (:`Triggered`
    (if (`self.NotCrushed`)
      (`self.AddMovementInput` (`self.GetActorForwardVector`) ActionValue)
      (`SceneComponent.K2_AddWorldRotation` (`self.Sphere1`) (`KismetMathLibrary.MakeRotator` 0.0 (* ActionValue -10.0)) false false))))

(event `self.Sphere.OnComponentBeginOverlap`
  (params (OverlappedComponent :type "PrimitiveComponent Object Reference") (OtherActor :type "Actor Object Reference") (OtherComp :type "PrimitiveComponent Object Reference") (OtherBodyIndex :type Integer) (bFromSweep :type Boolean) (SweepResult :type "HitResult Structure (by ref)"))
  (cast `/Game/CarDodge/BP_Car` OtherActor)
  (set `self.NotCrushed` false)
  (`SceneComponent.SetWorldScale3D` (`self.Sphere`) (1.0 1.0 0.01))
  (`SceneComponent.K2_SetWorldRotation` :`self` (`self.Sphere1`)))

(event `/Game/I_ToggeableDebugVisualization.ToggleDebugVisualization`
  (if (`self.ToggleOn`)
    (`SceneComponent.SetHiddenInGame` (`self.Arrow`) true false)
    (`SceneComponent.SetHiddenInGame` (`self.Sphere`) true false)
    (set `self.ToggleOn` false)
    (else
      (`SceneComponent.SetHiddenInGame` (`self.Arrow`) false false)
      (`SceneComponent.SetHiddenInGame` (`self.Sphere`) false false)
      (set `self.ToggleOn` true))))

(fn `UserConstructionScript`)