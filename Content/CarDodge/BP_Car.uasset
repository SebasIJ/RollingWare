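; BP_Car is a moving car actor for the CarDodge game that drives forward and destroys itself ten seconds after spawning.
; BeginPlay picks a random speed, and Tick offsets the Box component along its local X axis by that speed, scaled by delta time.
; Overlapping a BP_CarCheck sets an OutOfBounds flag, which is not read here.
; A ToggleDebugVisualization event shows or hides the Arrow and Box components.
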(event `self.ReceiveBeginPlay`
  (set `self.Speed` (`KismetMathLibrary.RandomFloatInRange` 1500.0 2200.0))
  (`KismetSystemLibrary.K2_SetTimerDelegate` (delegate `SelfDestruct`) 10.0))

(event `SelfDestruct`
  (`self.K2_DestroyActor`))

(event `self.ReceiveTick`
  (params (DeltaSeconds :type "Float (single-precision)"))
  (`SceneComponent.K2_AddLocalOffset` (`self.Box`) (`KismetMathLibrary.MakeVector` (* DeltaSeconds (`self.Speed`))) false false))

(event `self.Box.OnComponentBeginOverlap`
  (params (OverlappedComponent :type "PrimitiveComponent Object Reference") (OtherActor :type "Actor Object Reference") (OtherComp :type "PrimitiveComponent Object Reference") (OtherBodyIndex :type Integer) (bFromSweep :type Boolean) (SweepResult :type "HitResult Structure (by ref)"))
  (cast `/Game/CarDodge/BP_CarCheck` OtherActor)
  (set `self.OutOfBounds` true))

(event `/Game/I_ToggeableDebugVisualization.ToggleDebugVisualization`
  (if (`self.ToggleOn`)
    (`SceneComponent.SetHiddenInGame` (`self.Arrow`) true false)
    (`SceneComponent.SetHiddenInGame` (`self.Box`) true false)
    (set `self.ToggleOn` false)
    (else
      (`SceneComponent.SetHiddenInGame` (`self.Arrow`) false false)
      (`SceneComponent.SetHiddenInGame` (`self.Box`) false false)
      (set `self.ToggleOn` true))))

(fn `UserConstructionScript`)