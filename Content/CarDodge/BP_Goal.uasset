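; BP_Goal is the goal trigger for the CarDodge minigame, marking a win when the player's car reaches it.
; On BeginPlay it clears WinMinigame on MainGameMode and moves its Box to a random Y position, keeping X and Z.
; When BP_MCCarDodge overlaps the Box, it sets WinMinigame, prints "Win", and plays a 2D win sound guarded to fire only once.
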(event `self.ReceiveBeginPlay`
  (bind (_returnvalue_x _returnvalue_y _returnvalue_z) (`KismetMathLibrary.BreakVector` (`SceneComponent.K2_GetComponentLocation` (`self.Box`))))
  (bind _asmain_game_mode (cast `/Game/MainGameMode` (`GameplayStatics.GetGameMode`)))
  (set `/Game/MainGameMode.WinMinigame` false _asmain_game_mode)
  (`SceneComponent.K2_SetWorldLocation` (`self.Box`) (`KismetMathLibrary.MakeVector` _returnvalue_x (`KismetMathLibrary.RandomFloatInRange` -1000.0 1000.0) _returnvalue_z) false false))

(event `self.Box.OnComponentBeginOverlap`
  (params (OverlappedComponent :type "PrimitiveComponent Object Reference") (OtherActor :type "Actor Object Reference") (OtherComp :type "PrimitiveComponent Object Reference") (OtherBodyIndex :type Integer) (bFromSweep :type Boolean) (SweepResult :type "HitResult Structure (by ref)"))
  (cast `/Game/CarDodge/BP_MCCarDodge` OtherActor)
  (bind _asmain_game_mode (cast `/Game/MainGameMode` (`GameplayStatics.GetGameMode`)))
  (set `/Game/MainGameMode.WinMinigame` true _asmain_game_mode)
  (`KismetSystemLibrary.PrintString` "Win")
  (if (not (`self.PlayedSound`))
    (`GameplayStatics.PlaySound2D` "/Game/Sound/WAV_Win.WAV_Win" 1.0 1.0 0.0 null null)
    (set `self.PlayedSound` true)))

(fn `UserConstructionScript`)