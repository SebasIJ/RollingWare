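; BP_BatBall is the ball actor in the BatHit minigame, which travels along -X at a random speed rolled and printed on BeginPlay.
; Tick offsets Sphere and spins Sphere1 around pitch until the Hit flag, not set true in this file, becomes true.
; Once hit, the ball flies toward +X and +Z with reversed spin, sets WinMinigame on MainGameMode and plays the win sound once.
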(event `self.ReceiveBeginPlay`
  (bind _output_get (set `self.Speed` (`KismetMathLibrary.RandomFloatInRange` 450.0 1000.0)))
  (`KismetSystemLibrary.PrintString` (`KismetStringLibrary.BuildString_Double` "" "" _output_get))
  (set `self.Hit` false))

(event `self.ReceiveTick`
  (params (DeltaSeconds :type "Float (single-precision)"))
  (bind _returnvalue (* (* (`self.Speed`) DeltaSeconds) 2.0))
  (if (`self.Hit`)
    (set `self.Speed` 500.0)
    (`SceneComponent.K2_AddWorldOffset` (`self.Sphere`) (`KismetMathLibrary.MakeVector` _returnvalue 0.0 _returnvalue) false false)
    (`SceneComponent.K2_AddWorldRotation` (`self.Sphere1`) (`KismetMathLibrary.MakeRotator` 0.0 (* (`self.Speed`) -2.0)) false false)
    (bind _asmain_game_mode (cast `/Game/MainGameMode` (`GameplayStatics.GetGameMode`)))
    (set `/Game/MainGameMode.WinMinigame` true _asmain_game_mode)
    (if (not (`self.SoundPlayed`))
      (`GameplayStatics.PlaySound2D` "/Game/Sound/WAV_Win.WAV_Win" 1.0 1.0 0.0 null null)
      (set `self.SoundPlayed` true))
    (else
      (`SceneComponent.K2_AddWorldOffset` (`self.Sphere`) (`KismetMathLibrary.MakeVector` (* (* (`self.Speed`) DeltaSeconds) -1.0)) false false)
      (`SceneComponent.K2_AddWorldRotation` (`self.Sphere1`) (`KismetMathLibrary.MakeRotator` 0.0 (* (`self.Speed`) DeltaSeconds)) false false))))

(fn `UserConstructionScript`)