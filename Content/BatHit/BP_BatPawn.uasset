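; BP_BatPawn is the player-controlled bat pawn in a bat-and-ball hitting game, swung with the IA_SpaceAction input.
; Each press starts a swing that Tick advances by a fixed yaw step per frame, completing one frame-rate-dependent full turn before resetting.
; Box overlap events track BP_BatBall, and a ball overlapping during a swing gets its Hit flag set.
; ToggleDebugVisualization shows or hides the Arrow and Box.
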(event `self.ReceiveBeginPlay`
  (bind _asplayer_controller (cast `PlayerController` (`self.GetController`)))
  (`EnhancedInputSubsystemInterface.AddMappingContext` (pcsubsystem `EnhancedInputLocalPlayerSubsystem` _asplayer_controller) "/Game/Input/InputMapping.InputMapping" 0 (struct))
  (`KismetSystemLibrary.PrintString` "BatReady"))

(event `self.ReceiveTick`
  (params (DeltaSeconds :type "Float (single-precision)"))
  (if (`self.Hitting`)
    (`SceneComponent.K2_AddWorldRotation` (`self.Bat`) (`KismetMathLibrary.MakeRotator` 0.0 0.0 -20.0) false false)
    (if (`self.BallOverlap`)
      (bind _asbp_bat_ball (cast `/Game/BatHit/BP_BatBall` (stale `self.Box.OnComponentBeginOverlap` OtherActor)))
      (if (`self.Hitting`)
        (set `/Game/BatHit/BP_BatBall.Hit` true _asbp_bat_ball)
        (bind _result (`/Engine/EditorBlueprintResources/StandardMacros.IncrementInt` (`self.HitTime`) :!label _label)
          (:`  `
            (if (== _result 18)
              (set `self.Hitting` false)
              (set `self.HitTime` 0)))))
      (else
        (goto _label)))))

(event `EnhancedInput|/Game/Input/IA_SpaceAction`
  (params (ActionValue :type Boolean) (ElapsedSeconds :type "Float (double-precision)") (TriggeredSeconds :type "Float (double-precision)") (InputAction :type "InputAction Object Reference" :default "/Game/Input/IA_SpaceAction.IA_SpaceAction"))
  (:`Started`
    (set `self.Hitting` true)))

(event `self.Box.OnComponentBeginOverlap`
  (params (OverlappedComponent :type "PrimitiveComponent Object Reference") (OtherActor :type "Actor Object Reference") (OtherComp :type "PrimitiveComponent Object Reference") (OtherBodyIndex :type Integer) (bFromSweep :type Boolean) (SweepResult :type "HitResult Structure (by ref)"))
  (cast `/Game/BatHit/BP_BatBall` OtherActor)
  (set `self.BallOverlap` true))

(event `self.Box.OnComponentEndOverlap`
  (params (OverlappedComponent :type "PrimitiveComponent Object Reference") (OtherActor :type "Actor Object Reference") (OtherComp :type "PrimitiveComponent Object Reference") (OtherBodyIndex :type Integer))
  (cast `/Game/BatHit/BP_BatBall` OtherActor)
  (set `self.BallOverlap` false))

(event `/Game/I_ToggeableDebugVisualization.ToggleDebugVisualization`
  (if (`self.ToggleOn`)
    (`SceneComponent.SetHiddenInGame` (`self.Arrow`) true false)
    (`SceneComponent.SetHiddenInGame` (`self.Box`) true false)
    (set `self.ToggleOn` false)
    (else
      (`SceneComponent.SetHiddenInGame` (`self.Arrow`) false false)
      (`SceneComponent.SetHiddenInGame` (`self.Box`) false false)
      (set `self.ToggleOn` true))))

(fn `UserConstructionScript`)